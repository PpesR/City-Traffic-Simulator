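; City traffic light Blueprint that cycles red, green and yellow, either on its own or paired with an opposite light.
; A light without a valid OppositeLight runs an endless Delay loop on BeginPlay, stepping LightState through red, yellow, green and yellow.
; A linked light reads OppositeLight's state instead, swapping red and green while sharing yellow.
; Tick sets the EmissionColor parameter on LightBox's materials every frame.
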(event EventBeginPlay
  (Utilities|IsValid (Variables|Default|GetOppositeLight)
    (:Is%20Not%20Valid
      (Variables|Default|SetLightState 1 :!label _label)
      (Utilities|FlowControl|Delay 1e+01)
      (Variables|Default|SetLightState 3)
      (Utilities|FlowControl|Delay 2.0)
      (Variables|Default|SetLightState 2)
      (Utilities|FlowControl|Delay 1e+01)
      (Variables|Default|SetLightState 4)
      (Utilities|FlowControl|Delay 2.0)
      (goto _label))))

(event EventTick
  (params (DeltaSeconds :type Float%20%28single-precision%29))
  (bind _lightbox (Variables|Default|GetLightBox))
  (bind _oppositelight (Variables|Default|GetOppositeLight))
  (bind _lightbox_2 (Variables|Default|GetLightBox))
  (bind _lightstate (Variables|Default|GetLightState))
  (bind _lightstate_2 (Variables|TrafficLight_BP_C|GetLightState _oppositelight))
  (Utilities|IsValid (Variables|Default|GetOppositeLight)
    (:Is%20Valid
      (if (== _lightstate_2 1)
        (Rendering|Material|SetVectorParameterValueonMaterials _lightbox_2 "EmissionColor" (Math|Conversions|ToVector(LinearColor) (Math|Color|SelectColor :A "(R=0.000000,G=0.192157,B=0.000000,A=1.000000)" :bPickA true)))
        (elif (< _lightstate_2 3)
          (Rendering|Material|SetVectorParameterValueonMaterials _lightbox_2 "EmissionColor" (Math|Conversions|ToVector(LinearColor) (Math|Color|SelectColor :A "(R=1.000000,G=0.000000,B=0.000000,A=1.000000)" :bPickA true)))
          (else
            (Rendering|Material|SetVectorParameterValueonMaterials _lightbox_2 "EmissionColor" (Math|Conversions|ToVector(LinearColor) (Math|Color|SelectColor :A "(R=1.000000,G=0.938499,B=0.000000,A=1.000000)" :bPickA true)))))))
    (:Is%20Not%20Valid
      (if (== _lightstate 1)
        (Rendering|Material|SetVectorParameterValueonMaterials _lightbox "EmissionColor" (Math|Conversions|ToVector(LinearColor) (Math|Color|SelectColor :A "(R=1.000000,G=0.000000,B=0.000000,A=1.000000)" :bPickA true)))
        (elif (< _lightstate 3)
          (Rendering|Material|SetVectorParameterValueonMaterials _lightbox "EmissionColor" (Math|Conversions|ToVector(LinearColor) (Math|Color|SelectColor :A "(R=0.000000,G=0.192157,B=0.000000,A=1.000000)" :bPickA true)))
          (else
            (Rendering|Material|SetVectorParameterValueonMaterials _lightbox "EmissionColor" (Math|Conversions|ToVector(LinearColor) (Math|Color|SelectColor :A "(R=1.000000,G=0.943203,B=0.000000,A=1.000000)" :bPickA true)))))))))

(fn ConstructionScript)